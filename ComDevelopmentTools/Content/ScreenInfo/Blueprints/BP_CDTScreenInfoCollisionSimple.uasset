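; Screen info Blueprint that flags components with simple collision, going by its name as part of a CDT screen info set.
; It rejects every actor in CheckActor, so matching happens only per component.
; CheckComponent passes a primitive component only when its collision is enabled and the HasCollisionSimple helper reports simple collision.
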(fn `CheckActor`
  (params (Actor :type "Actor Object Reference"))
  (returns (ReturnValue :type Boolean))
  (return false))

(fn `CheckComponent`
  (params (Actor :type "Actor Object Reference") (Component :type "ActorComponent Object Reference"))
  (returns (ReturnValue :type Boolean))
  (bind _asprimitive_component (cast `PrimitiveComponent` Component)
    (:`then`
      (if (`PrimitiveComponent.K2_IsCollisionEnabled` _asprimitive_component)
        (bind _returnvalue (`CDTBPFLUtility.HasCollisionSimple` _asprimitive_component))
        (return _returnvalue)
        (else
          (return false))))
    (:`CastFailed`
      (return false))))

(fn `UserConstructionScript`
  (`parent.UserConstructionScript`))