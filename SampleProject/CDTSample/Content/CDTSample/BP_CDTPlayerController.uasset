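; Player controller for the CDT sample that toggles debug screen-info overlays and reports draw call counts.
; On BeginPlay it spawns seven ScreenInfo actors covering collision variants, overlap events, dynamic shadows, max LOD and tick, and number keys toggle each through a shared InputScreenInfo function.
; It also enables the SceneRendering stat group undisplayed until EndPlay, so Q can print the average MeshDrawCalls value.
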(event `self.ReceiveBeginPlay`
  (`|ExecutionSequence`
    (:`then_0`
      ;[0.3812 0.4441 1] ScreenInfo: Collision
      (bind _returnvalue (`|SpawnActorFromClass` "/ComDevelopmentTools/ScreenInfo/Blueprints/BP_CDTScreenInfoCollision.BP_CDTScreenInfoCollision_C" (`KismetMathLibrary.MakeTransform` (0.0 0.0 0.0)) "Undefined" "OverrideRootScale" null 5 null))
      ;[0.3812 0.4441 1] ScreenInfo: Collision Simple
      (bind _returnvalue_2 (`|SpawnActorFromClass` "/ComDevelopmentTools/ScreenInfo/Blueprints/BP_CDTScreenInfoCollisionSimple.BP_CDTScreenInfoCollisionSimple_C" (`KismetMathLibrary.MakeTransform` (0.0 0.0 0.0)) "Undefined" "OverrideRootScale" null 5 null))
      ;[0.3812 0.4441 1] ScreenInfo: Collision Complex
      (bind _returnvalue_3 (`|SpawnActorFromClass` "/ComDevelopmentTools/ScreenInfo/Blueprints/BP_CDTScreenInfoCollisionSimpleComplex.BP_CDTScreenInfoCollisionSimpleComplex_C" (`KismetMathLibrary.MakeTransform` (0.0 0.0 0.0)) "Undefined" "OverrideRootScale" null 5 null))
      ;[0.3812 0.4441 1] ScreenInfo: Overlap Events
      (bind _returnvalue_4 (`|SpawnActorFromClass` "/ComDevelopmentTools/ScreenInfo/Blueprints/BP_CDTScreenInfoOverlapEvents.BP_CDTScreenInfoOverlapEvents_C" (`KismetMathLibrary.MakeTransform` (0.0 0.0 0.0)) "Undefined" "OverrideRootScale" null 5 null))
      ;[0.3812 0.4441 1] ScreenInfo: Dynamic Shadow
      (bind _returnvalue_5 (`|SpawnActorFromClass` "/ComDevelopmentTools/ScreenInfo/Blueprints/BP_CDTScreenInfoDynamicShadow.BP_CDTScreenInfoDynamicShadow_C" (`KismetMathLibrary.MakeTransform` (0.0 0.0 0.0)) "Undefined" "OverrideRootScale" null 5 null))
      ;[0.3812 0.4441 1] ScreenInfo: LOD Max
      (bind _returnvalue_6 (`|SpawnActorFromClass` "/ComDevelopmentTools/ScreenInfo/Blueprints/BP_CDTScreenInfoLODMax.BP_CDTScreenInfoLODMax_C" (`KismetMathLibrary.MakeTransform` (0.0 0.0 0.0)) "Undefined" "OverrideRootScale" null 5 null))
      ;[0.3812 0.4441 1] ScreenInfo: Tick
      (bind _returnvalue_7 (`|SpawnActorFromClass` "/ComDevelopmentTools/ScreenInfo/Blueprints/BP_CDTScreenInfoTick.BP_CDTScreenInfoTick_C" (`KismetMathLibrary.MakeTransform` (0.0 0.0 0.0)) "Undefined" "OverrideRootScale" null 5 null)))
    (:`then_1`
      ;[0.2104 1 0.2948] Stat: Groupを有効に
      (`CDTBPFLStats.SetEnableStatGroup` "SceneRendering" true))))

(event `Key|One`
  (params (Key :type "Key Structure"))
  ;[0.3812 0.4441 1] ScreenInfo: Collision
  (:`Pressed`
    (`self.InputScreenInfo` (stale `self.ReceiveBeginPlay` _returnvalue))))

(event `Key|Two`
  (params (Key :type "Key Structure"))
  ;[0.3812 0.4441 1] ScreenInfo: Collision Simple
  (:`Pressed`
    (`self.InputScreenInfo` (stale `self.ReceiveBeginPlay` _returnvalue_2))))

(event `Key|Three`
  (params (Key :type "Key Structure"))
  ;[0.3812 0.4441 1] ScreenInfo: Collision Complex
  (:`Pressed`
    (`self.InputScreenInfo` (stale `self.ReceiveBeginPlay` _returnvalue_3))))

(event `Key|Four`
  (params (Key :type "Key Structure"))
  ;[0.3812 0.4441 1] ScreenInfo: Overlap Events
  (:`Pressed`
    (`self.InputScreenInfo` (stale `self.ReceiveBeginPlay` _returnvalue_4))))

(event `Key|Five`
  (params (Key :type "Key Structure"))
  ;[0.3812 0.4441 1] ScreenInfo: Dynamic Shadow
  (:`Pressed`
    (`self.InputScreenInfo` (stale `self.ReceiveBeginPlay` _returnvalue_5))))

(event `Key|Six`
  (params (Key :type "Key Structure"))
  ;[0.3812 0.4441 1] ScreenInfo: LOD Max
  (:`Pressed`
    (`self.InputScreenInfo` (stale `self.ReceiveBeginPlay` _returnvalue_6))))

(event `Key|Seven`
  (params (Key :type "Key Structure"))
  ;[0.3812 0.4441 1] ScreenInfo: Tick
  (:`Pressed`
    (`self.InputScreenInfo` (stale `self.ReceiveBeginPlay` _returnvalue_7))))

(event `self.ReceiveEndPlay`
  (params (EndPlayReason :type "EEndPlayReason Enum" :default "Destroyed"))
  ;[0.2104 1 0.2948] Statを元に戻す
  (`CDTBPFLStats.SetEnableStatGroup` "SceneRendering"))

(event `Key|Q`
  (params (Key :type "Key Structure"))
  (:`Pressed`
    ;[0.2104 1 0.2948] DrawCallの数を取得
    (bind _returnvalue (`CDTBPFLStats.GetStatValueAverage` "MeshDrawCalls"))
    (`KismetSystemLibrary.PrintString` (`KismetTextLibrary.Conv_TextToString` (`|FormatText` "DrawCall : {Num}" _returnvalue)))))

(fn `InputScreenInfo`
  (params (ScreenInfo :type "/ComDevelopmentTools/ScreenInfo/Blueprints/BP_CDTScreenInfoBase Object Reference"))
  (bind _screeninfo (`local.ScreenInfo`))
  (if (`CDTScreenInfoBase.IsEnabled` ScreenInfo)
    (`CDTScreenInfoBase.SetEnable` _screeninfo false)
    (else
      (`CDTScreenInfoBase.SetEnable` _screeninfo true))))

(fn `UserConstructionScript`)